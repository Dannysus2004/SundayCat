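; BP_Platforms is a platform that is solid only while the player character overlaps its Box volume.
; BeginPlay caches the player's BP_Character.
; Every Tick checks that overlap and switches the Cube's collision between query-and-physics and none.
; The Box begin and end overlap events only cast to BP_Character and take no further action.
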(event OnComponentBeginOverlap(Box)
  (params (OverlappedComponent :type Primitive%20Component%20Object%20Reference) (OtherActor :type Actor%20Object%20Reference) (OtherComp :type Primitive%20Component%20Object%20Reference) (OtherBodyIndex :type Integer) (bFromSweep :type Boolean) (SweepResult :type Hit%20Result%20Structure%20%28by%20ref%29))
  (Utilities|Casting|CastToBP_Character OtherActor))

(event OnComponentEndOverlap(Box)
  (params (OverlappedComponent :type Primitive%20Component%20Object%20Reference) (OtherActor :type Actor%20Object%20Reference) (OtherComp :type Primitive%20Component%20Object%20Reference) (OtherBodyIndex :type Integer))
  (Utilities|Casting|CastToBP_Character OtherActor))

(event EventBeginPlay
  (bind _asbp_character (Utilities|Casting|CastToBP_Character (Game|GetPlayerCharacter 0)))
  (Variables|Default|SetAs%20BP%20Character _asbp_character))

(event Collision|EventActorBeginOverlap
  (params (OtherActor :type Actor%20Object%20Reference)))

(event EventTick
  (params (DeltaSeconds :type Float%20%28single-precision%29))
  (bind _cube (Variables|Default|GetCube))
  (if (Collision|IsOverlappingActor (Variables|Default|GetBox) (Variables|Default|GetAs%20BP%20Character) :!class /Script/Engine.PrimitiveComponent)
    (Collision|SetCollisionEnabled _cube "QueryAndPhysics")
    (else
      (Collision|SetCollisionEnabled _cube "NoCollision"))))

(fn ConstructionScript)