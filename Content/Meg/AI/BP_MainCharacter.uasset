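; BP_MainCharacter is a Character Blueprint in the AI folder that carries a spline and exposes walk speed control.
; On BeginPlay it caches the world locations of the spline's first six points in separate variables, which this Blueprint does not itself use.
; UpdateWalkSpeed sets the movement component's max walk speed to a passed value.
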(event EventBeginPlay
  (bind _spline (Variables|Default|GetSpline))
  (Variables|Default|SetSplineP0 (Spline|GetLocationatSplinePoint _spline 0 "World"))
  (Variables|Default|SetSplinep1 (Spline|GetLocationatSplinePoint _spline 1 "World"))
  (Variables|Default|SetSplineP2 (Spline|GetLocationatSplinePoint _spline 2 "World"))
  (Variables|Default|SetSplinep3 (Spline|GetLocationatSplinePoint _spline 3 "World"))
  (Variables|Default|SetSplineP4 (Spline|GetLocationatSplinePoint _spline 4 "World"))
  (Variables|Default|SetSplineP5 (Spline|GetLocationatSplinePoint _spline 5 "World")))

(fn ConstructionScript)

(fn UpdateWalkSpeed
  (params (NewWalkSpeed :type Float%20%28double-precision%29))
  (Variables|/Script/Engine.CharacterMovementComponent|SetMaxWalkSpeed (Variables|Character|GetCharacterMovement) NewWalkSpeed))