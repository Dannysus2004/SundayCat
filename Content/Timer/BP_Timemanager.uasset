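; BP_Timemanager is a game clock that decides when tasks and disruptions like coffee, keys, alarm, clothes, sleep and shower are available.
; From BeginPlay, a self-calling TimerLoop increments CurrentTime after each one-second Delay and runs every task event.
; Each event uses TimeAvailability to test its inclusive time window, stores a boolean and debug-prints it.
; ShowerTime writes to IsSleeping, overwriting SleepTime's result on every tick of the loop.
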(event Custom|SleepTime
  (bind _is_available (CallFunction|TimeAvailability (Variables|Default|GetCurrent%20Time) 0.0 6e+01))
  (bind _output_get (Variables|Default|SetIsSleeping _is_available))
  (Development|PrintString (Utilities|String|ToString(Boolean) _output_get) true true "(R=1.000000,G=0.867539,B=0.000000,A=1.000000)"))

(event Custom|Timer%20Loop
  (bind _output_get (Variables|Default|SetCurrent%20Time (+ (Variables|Default|GetCurrent%20Time) 1.0)))
  (Development|PrintString (Utilities|String|ToString(Float) _output_get))
  (Utilities|FlowControl|Delay 1.0)
  ;[1 1 1] Tasks/Disruptions
  (CallFunction|Coffee)
  (CallFunction|Keys)
  (CallFunction|Alarm)
  (CallFunction|Clothes)
  (CallFunction|SleepTime)
  (CallFunction|ShowerTime)
  (CallFunction|TimerLoop))

(event Custom|Alarm
  ;[1 1 1] Interactables
  (bind _is_available (CallFunction|TimeAvailability (Variables|Default|GetCurrent%20Time) 0.0 6e+01))
  (bind _output_get (Variables|Default|SetAlarm%20Available _is_available))
  (Development|PrintString (Utilities|String|ToString(Boolean) _output_get) true true "(R=0.000000,G=0.040459,B=1.000000,A=1.000000)"))

(event Custom|Coffee
  ;[1 1 1] Interactables
  (bind _is_available (CallFunction|TimeAvailability (Variables|Default|GetCurrent%20Time) 6e+01 1.2e+02))
  (bind _output_get (Variables|Default|SetCoffee%20Avaible _is_available))
  (Development|PrintString (Utilities|String|ToString(Boolean) _output_get)))

(event Custom|ShowerTime
  (bind _is_available (CallFunction|TimeAvailability (Variables|Default|GetCurrent%20Time) 1.2e+02 1.4e+02))
  (bind _output_get (Variables|Default|SetIsSleeping _is_available))
  (Development|PrintString (Utilities|String|ToString(Boolean) _output_get) true true "(R=1.000000,G=0.062383,B=0.000000,A=1.000000)"))

(event Custom|Keys
  ;[1 1 1] Interactables
  (bind _is_available (CallFunction|TimeAvailability (Variables|Default|GetCurrent%20Time) 0.0 1.8e+02))
  (bind _output_get (Variables|Default|SetKeys%20Available _is_available))
  (Development|PrintString (Utilities|String|ToString(Boolean) _output_get) true true "(R=0.112749,G=1.000000,B=0.025833,A=1.000000)"))

(event Custom|Clothes
  ;[1 1 1] Interactables
  (bind _is_available (CallFunction|TimeAvailability (Variables|Default|GetCurrent%20Time) 1.2e+02 1.4e+02))
  (bind _output_get (Variables|Default|SetClothes%20Available _is_available))
  (Development|PrintString (Utilities|String|ToString(Boolean) _output_get) true true "(R=1.000000,G=0.147550,B=0.695255,A=1.000000)"))

(event EventBeginPlay
  (Variables|Default|SetCurrent%20Time 0.0)
  (CallFunction|TimerLoop))

(fn ConstructionScript)

(fn TimeAvailability
  (params (Current%20Time :type Float%20%28double-precision%29) (Available%20From :type Float%20%28double-precision%29) (Available%20Until :type Float%20%28double-precision%29))
  (if (and (>= Current%20Time Available%20From) (<= Current%20Time Available%20Until))
    (return true)
    (else
      (return false))))